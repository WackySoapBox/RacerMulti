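; Lobby game mode that shows the lobby UI and tracks joining and leaving player controllers against the session's connection limit.
; BeginPlay creates WG_Lobby from the fetched session settings.
; Once the limit is reached, PostLogin kicks controllers indexed above it as "Serveur complet" (server full), then notifies the widget of the newcomer.
; A delayed kick-and-UpdateSession variant is left unconnected.
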(event `self.ReceiveBeginPlay`
  (bind (_numconnections _numprivateconnections _bislan _bisdedicated _ballowinvites _ballowjoininprogress _bisanticheatenabled _builduniqueid _extrasettings) (`AdvancedSessionsLibrary.GetSessionSettings`)
    (:`OnSuccess`
      (bind _returnvalue (`|CreateWidget` "/Game/Multiplayer/Lobby/WG_Lobby.WG_Lobby_C" (`GameplayStatics.GetPlayerController` 0) _extrasettings _numconnections null))
      (`UserWidget.AddToViewport` _returnvalue 0))))

(event `self.HandleStartingNewPlayer`
  (params (NewPlayer :type "PlayerController Object Reference"))
  ;[1 1 1] With Player check
)

(event `self.K2_PostLogin`
  (params (NewPlayer :type "PlayerController Object Reference"))
  (bind _playercontrollers (`self.PlayerControllers`))
  (`KismetArrayLibrary.Array_AddUnique` (`self.PlayerControllers`) NewPlayer)
  (bind _numconnections (`AdvancedSessionsLibrary.GetSessionSettings`)
    (:`OnSuccess`
      (if (not (< (`KismetArrayLibrary.Array_Length` _playercontrollers) _numconnections))
        (bind (_arrayindex _arrayelement) (`/Engine/EditorBlueprintResources/StandardMacros.ReverseForEachLoop` _playercontrollers)
          (:`LoopBody`
            (if (> _arrayindex _numconnections)
              (`AdvancedSessionsLibrary.KickPlayer` _arrayelement "Serveur complet")))
          (:`Completed`
            (bind _foundwidgets (`WidgetBlueprintLibrary.GetAllWidgetsOfClass` "/Game/Multiplayer/Lobby/WG_Lobby.WG_Lobby_C"))
            (`/Game/Multiplayer/Lobby/WG_Lobby.NewPlayerHere` (`|GetArrayItem` _foundwidgets) NewPlayer)))))))

(event `self.K2_OnLogout`
  (params (ExitingController :type "Controller Object Reference"))
  (bind _asplayer_controller (cast `PlayerController` ExitingController))
  (`KismetArrayLibrary.Array_RemoveItem` (`self.PlayerControllers`) _asplayer_controller))

(fn `UserConstructionScript`)