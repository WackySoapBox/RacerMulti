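; Finish line actor for split-screen races that scores each player vehicle overlapping it and freezes it.
; Placement points follow the order vehicles are added to the finished list.
; An element score tallies the vehicle's visible elements by set, matching mesh names, and sums the squared counts.
; Once all vehicles finish, it plays a final sound and replaces all widgets with the next-race selection screen, which calculates scores.
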(event `self.ReceiveActorBeginOverlap`
  (params (OtherActor :type "Actor Object Reference"))
  (bind _returnvalue (`GameplayStatics.GetPlayerController` 0))
  (if (`self.ActorHasTag` OtherActor "Player")
    (bind _aspc_vehicle (cast `/Game/Jules/Pawn/PC_Vehicle` OtherActor))
    (set `self.PcVehicle` _aspc_vehicle)
    (set `self.PlayerController` (`Pawn.GetLocalViewingPlayerController` _aspc_vehicle))
    (`self.CalculateElementScore`
      (:`Output`
        (bind _asgm_split_screen (cast `/Game/Multiplayer/SplitScreen/GM_SplitScreen` (`GameplayStatics.GetGameMode`)))
        (bind _returnvalue_2 (`KismetArrayLibrary.Array_AddUnique` (`self.PlayerFini`) (`self.PcVehicle`)))
        (set `/Game/Jules/Pawn/PC_Vehicle.ScorePlace` (select `int` _returnvalue_2 :`0` 50 :`1` 46 :`2` 42 :`3` 38) (`self.PcVehicle`))
        (set `/Game/Jules/Pawn/PC_Vehicle.freezeStart` true (`self.PcVehicle`))
        (if (>= (`KismetArrayLibrary.Array_Length` (`self.PlayerFini`)) (`BlueprintMapLibrary.Map_Length` (`/Game/Multiplayer/SplitScreen/GM_SplitScreen.VehiculesPosition` _asgm_split_screen)))
          (`GameplayStatics.SpawnSound2D` "/Game/Jules/SoundDesign/SoundCues/SonFinal.SonFinal" 1.0 1.0 0.0 null)
          (`WidgetLayoutLibrary.RemoveAllWidgets`)
          (set `PlayerController.bShowMouseCursor` true _returnvalue)
          (bind _returnvalue_3 (`|CreateWidget` "/Game/Multiplayer/RacingFrameWork/WG_ChooseNextRace.WG_ChooseNextRace_C" _returnvalue))
          (`UserWidget.AddToViewport` _returnvalue_3 0)
          (`/Game/Multiplayer/RacingFrameWork/WG_ChooseNextRace.CalculateScore` _returnvalue_3))))))

(fn `UserConstructionScript`)