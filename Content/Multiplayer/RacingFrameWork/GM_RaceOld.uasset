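; GM_RaceOld is a race game mode that handles the start countdown and the end-of-race screen.
; On BeginPlay it waits a countdown delay, then a one-shot timer fires GameStart, which destroys every actor tagged "Barriere".
; EndRace shows the WG_ChooseNextRace widget without using its HasWin input, and FinishRace is an empty stub.
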(event `self.ReceiveBeginPlay`
  (`self.Start Countdown`))

(event `Start Countdown`
  (`KismetSystemLibrary.Delay` (`self.StartCountDownDuration`))
  (`KismetSystemLibrary.K2_SetTimerDelegate` (delegate `Game Start`) (`self.StartTimerDuration`)))

(event `Game Start`
  (bind _outactors (`GameplayStatics.GetAllActorsWithTag` "Barriere"))
  (for _array_element _outactors
    (`self.K2_DestroyActor` _array_element)))

(event `FinishRace`)

(event `EndRace`
  (params (hasWin :type Boolean))
  (bind _returnvalue (`|CreateWidget` "/Game/Multiplayer/RacingFrameWork/WG_ChooseNextRace.WG_ChooseNextRace_C"))
  (`UserWidget.AddToViewport` _returnvalue 0))

(fn `UserConstructionScript`)