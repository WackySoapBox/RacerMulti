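; Race game mode for multiplayer that spawns racers at numbered player starts by their index in GI_Racer's controller array.
; StartCountDown waits, then times StartRace, which removes start barriers and unfreezes PC_Vehicle instances.
; When all players finish, it shows the next-race widget on player 0 and later freezes the last finisher.
; The session player-count check that would kick extras and trigger the countdown is disconnected.
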(event `self.HandleStartingNewPlayer`
  (params (NewPlayer :type "PlayerController Object Reference"))
  ;[0.4855 1 0.8167] Connection et spawn des joueurs
  (`KismetArrayLibrary.Array_AddUnique` (`self.PlayerControllers`) NewPlayer)
  (`KismetSystemLibrary.RetriggerableDelay` 0.2))

(event `self.ReceiveBeginPlay`
  ;[1 1 1] Begin play
)

(event `SetupRace`)

(event `StartCountDown`
  ;[1 1 1] Comment
  (`KismetSystemLibrary.Delay` (`self.StartCountDownDuration`))
  (`KismetSystemLibrary.K2_SetTimerDelegate` (delegate `StartRace`) (`self.StartTimerDuration`)))

(event `StartRace`
  ;[1 1 1] Comment
  (bind _outactors (`GameplayStatics.GetAllActorsWithTag` "BarriereStart"))
  (for _array_element _outactors
    (`self.K2_DestroyActor` _array_element))
  (bind _outactors_2 (`GameplayStatics.GetAllActorsOfClass` "/Script/Engine.PlayerController"))
  (set `self.PlayerControllers` _outactors_2)
  (bind _outactors_3 (`GameplayStatics.GetAllActorsOfClass` "/Game/Jules/Pawn/PC_Vehicle.PC_Vehicle_C"))
  (for _array_element_2 _outactors_3
    (set `/Game/Jules/Pawn/PC_Vehicle.freezeStart` false _array_element_2)))

(event `PlayerFinishRace`
  (params (playerController :type "PlayerController Object Reference") (PC_Vehicule :type "/Game/Jules/Pawn/PC_Vehicle Object Reference"))
  ;[1 1 1] Comment
  (set `self.NumPlayerHasFinished` (`KismetMathLibrary.Conv_Int64ToInt` (+ (`self.NumPlayerHasFinished`) 1)))
  (if (== (`KismetArrayLibrary.Array_Length` (`self.PlayerControllers`)) (`self.NumPlayerHasFinished`))
    (`self.EndRace`)
    (`KismetSystemLibrary.Delay` 2.0)
    (set `/Game/Jules/Pawn/PC_Vehicle.freezeStart` true PC_Vehicule)))

(event `EndRace`
  ;[1 1 1] Comment
  (bind _returnvalue (`GameplayStatics.GetCurrentLevelName` true))
  (bind _returnvalue_2 (`|CreateWidget` "/Game/Multiplayer/RacingFrameWork/WG_ChooseNextRace.WG_ChooseNextRace_C" null _returnvalue))
  (`UserWidget.AddToViewport` _returnvalue_2 0)
  (set `PlayerController.bShowMouseCursor` true (`GameplayStatics.GetPlayerController` 0)))

(fn `ChoosePlayerStart`
  (params (Player :type "Controller Object Reference"))
  (returns (ReturnValue :type "Actor Object Reference"))
  (bind _asgi_racer (cast `/Game/Multiplayer/Menu/GI_Racer` (`GameplayStatics.GetGameInstance`)))
  (for (_array_element _array_index) (`/Game/Multiplayer/Menu/GI_Racer.Array_PC` _asgi_racer)
    (if (== _array_element Player)
      (return (`self.K2_FindPlayerStart` Player (`KismetStringLibrary.Conv_IntToString` (+ _array_index 1)))))))

(fn `UserConstructionScript`)