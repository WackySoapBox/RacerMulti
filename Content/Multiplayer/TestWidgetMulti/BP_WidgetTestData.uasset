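; Multiplayer test Blueprint, apparently for widget testing, that holds an integer counter, DataI.
; Add1 calls OnServer, which calls Multicast to increment the counter, a server-to-multicast RPC relay going by the event names.
; Tick prints the current value to screen under a fixed key.
; DataI has an OnRep function, but it is empty.
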(event `self.ReceiveTick`
  (params (DeltaSeconds :type "Float (single-precision)"))
  (`KismetSystemLibrary.PrintString` (`KismetStringLibrary.Conv_IntToString` (`self.Data_I`)) true true (struct :`G` 0.66 :`B` 1.0 :`A` 1.0) 32.0 "blzlblzllgnlfdfg"))

(event `Add 1`
  (`self.on server`))

(event `multicast`
  (set `self.Data_I` (+ (`self.Data_I`) 1)))

(event `on server`
  (`self.multicast`))

(fn `OnRep_Data_I`)

(fn `UserConstructionScript`)