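; Game mode for multiplayer Circuit 1 that enforces the session's player limit and spawns each player's test suspension pawn.
; HandleStartingNewPlayer collects controllers, then after a retriggerable delay reads session settings and kicks any excess players.
; Once the expected count is reached, it updates the session, then spawns and possesses a pawn at each player's numbered start.
; PostLogin kicks every player logging in as too late to join.
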(event `self.HandleStartingNewPlayer`
  (params (NewPlayer :type "PlayerController Object Reference"))
  ;[1 1 1] With Player check
  (`KismetArrayLibrary.Array_AddUnique` (`self.PlayerControllers`) NewPlayer)
  (`KismetSystemLibrary.RetriggerableDelay` 0.2)
  (bind (_numconnections _numprivateconnections _bislan _bisdedicated _ballowinvites _ballowjoininprogress _bisanticheatenabled _builduniqueid _extrasettings) (`AdvancedSessionsLibrary.GetSessionSettings`)
    (:`OnSuccess`
      (if (> (`KismetArrayLibrary.Array_Length` (`GameStateBase.PlayerArray` (`GameplayStatics.GetGameState`))) _numconnections)
        (bind (_arrayindex _arrayelement) (`/Engine/EditorBlueprintResources/StandardMacros.ReverseForEachLoop` (`self.PlayerControllers`))
          (:`LoopBody`
            (if (>= _arrayindex _numconnections)
              (`AdvancedSessionsLibrary.KickPlayer` _arrayelement "Serveur complet")))
          (:`Completed`
            (`UpdateSessionCallbackProxyAdvanced.UpdateSession` _extrasettings _numconnections :!label _label
              (:`OnSuccess`
                (for (_array_element _array_index) (`self.PlayerControllers`)
                  (bind _returnvalue (`|SpawnActorFromClass` "/Game/Jules/Pawn/PC_Test_suspension.PC_Test_suspension_C" (`self.GetTransform` (`self.K2_FindPlayerStart` _array_element (`KismetStringLibrary.Conv_IntToString` (+ _array_index 1)))) "Undefined" "OverrideRootScale" null null))
                  (`Controller.Possess` _array_element _returnvalue))))))
        (elif (== (`KismetArrayLibrary.Array_Length` (`GameStateBase.PlayerArray` (`GameplayStatics.GetGameState`))) _numconnections)
          (goto _label))))))

(event `self.K2_PostLogin`
  (params (NewPlayer :type "PlayerController Object Reference"))
  (`AdvancedSessionsLibrary.KickPlayer` NewPlayer "In Game Too late"))

(fn `UserConstructionScript`)