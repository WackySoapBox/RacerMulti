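; Split-screen racing game mode that spawns the local players and releases the vehicles at the start.
; On BeginPlay it reads the player count from GI_Racer and runs chained, delayed CreatePlayer calls for two to four players.
; After a final short delay it clears FreezeStart on every PC_Vehicle, which the Space Bar also triggers directly.
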(event `Key|SpaceBar`
  (params (Key :type "Key Structure"))
  (:`Pressed`
    (bind _outactors (`GameplayStatics.GetAllActorsOfClass` "/Game/Jules/Pawn/PC_Vehicle.PC_Vehicle_C" :!label _label))
    (for _array_element _outactors
      (bind _aspc_vehicle (cast `/Game/Jules/Pawn/PC_Vehicle` _array_element))
      (set `/Game/Jules/Pawn/PC_Vehicle.freezeStart` false _aspc_vehicle))))

(event `self.ReceiveBeginPlay`
  (bind _asgi_racer (cast `/Game/Multiplayer/Menu/GI_Racer` (`GameplayStatics.GetGameInstance`)))
  (switch `int` (`/Game/Multiplayer/Menu/GI_Racer.SS_NumPlayer` _asgi_racer)
    (:`2`
      _)
    (:`3`
      (`KismetSystemLibrary.Delay` 0.2 :!label _label_2)
      (`GameplayStatics.CreatePlayer` -1))
    (:`4`
      (`KismetSystemLibrary.Delay` 0.2)
      (`GameplayStatics.CreatePlayer` -1)
      (goto _label_2)))
  (`KismetSystemLibrary.Delay` 0.2)
  (`GameplayStatics.CreatePlayer` -1)
  (`KismetSystemLibrary.Delay` 1.0)
  (goto _label))

(fn `UserConstructionScript`)