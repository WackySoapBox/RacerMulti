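; Test multiplayer GameMode that assigns pre-existing PWN_TestAllOnServer pawns to joining players.
; HandleStartingNewPlayer loops over those pawns and calls Possess on each unpossessed one, without breaking after the first.
; A disconnected, unused branch would instead wait until the session connection count matches PlayerArray, then give each PlayerController one free pawn and print the pairing.
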(event `self.ReceiveTick`
  (params (DeltaSeconds :type "Float (single-precision)")))

(event `self.HandleStartingNewPlayer`
  (params (NewPlayer :type "PlayerController Object Reference"))
  (bind _outactors (`GameplayStatics.GetAllActorsOfClass` "/Game/Multiplayer/TestMulti/PWN_TestAllOnServer.PWN_TestAllOnServer_C"))
  (for _array_element _outactors
    (if (not (`/Game/Multiplayer/TestMulti/PWN_TestAllOnServer.isPossessed` _array_element))
      (`Controller.Possess` NewPlayer _array_element))))

(fn `UserConstructionScript`)