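; Test multiplayer racing game mode that assigns player starts and releases the start freeze on vehicles.
; ChoosePlayerStart looks up the player's position in GI_Racer's ArrayPC and finds the start named by that one-based index, printing debug assignments.
; BeginPlay checks session connection count against that array once, without retrying.
; On a match, it waits briefly, then clears FreezeStart on every PC_Vehicle.
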(event `self.ReceiveBeginPlay`
  (bind _numconnections (`AdvancedSessionsLibrary.GetSessionSettings`)
    (:`OnSuccess`
      (bind _asgi_racer (cast `/Game/Multiplayer/Menu/GI_Racer` (`GameplayStatics.GetGameInstance`)))
      (if (== _numconnections (`KismetArrayLibrary.Array_Length` (`/Game/Multiplayer/Menu/GI_Racer.Array_PC` _asgi_racer)))
        (`KismetSystemLibrary.Delay` 1.0)
        (bind _outactors (`GameplayStatics.GetAllActorsOfClass` "/Game/Jules/Pawn/PC_Vehicle.PC_Vehicle_C"))
        (for _array_element _outactors
          (set `/Game/Jules/Pawn/PC_Vehicle.freezeStart` false _array_element))))))

(fn `ChoosePlayerStart`
  (params (Player :type "Controller Object Reference"))
  (returns (ReturnValue :type "Actor Object Reference"))
  (`KismetSystemLibrary.PrintString` (`KismetSystemLibrary.GetDisplayName` Player))
  (bind _asgi_racer (cast `/Game/Multiplayer/Menu/GI_Racer` (`GameplayStatics.GetGameInstance`)))
  (for (_array_element _array_index) (`/Game/Multiplayer/Menu/GI_Racer.Array_PC` _asgi_racer)
    (bind _returnvalue (+ _array_index 1))
    (`KismetSystemLibrary.PrintString` (`KismetStringLibrary.Concat_StrStr` "Player : " (`KismetSystemLibrary.GetDisplayName` _array_element) "| index spawn : " (`KismetStringLibrary.Conv_IntToString` _returnvalue)) true true (struct :`G` 0.66 :`B` 1.0 :`A` 1.0) 15.0 (`KismetStringLibrary.Conv_StringToName` (`KismetStringLibrary.Conv_IntToString` _array_index)))
    (if (== _array_element Player)
      (return (`self.K2_FindPlayerStart` Player (`KismetStringLibrary.Conv_IntToString` _returnvalue))))))

(fn `UserConstructionScript`)