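; Game mode for a prototype multiplayer lobby that shows the lobby widget on BeginPlay and tracks joining and leaving player controllers.
; After a short retriggerable delay on each join, it reads the session settings and kicks players beyond the connection count as "Serveur complet".
; It updates the session when the lobby is full or over capacity.
; The ServerTravel logic to LV_Circuit1 is disconnected, so it never starts the race.
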(event `self.ReceiveTick`
  (params (DeltaSeconds :type "Float (single-precision)")))

(event `self.K2_OnLogout`
  (params (ExitingController :type "Controller Object Reference"))
  (bind _asplayer_controller (cast `PlayerController` ExitingController))
  (`KismetArrayLibrary.Array_RemoveItem` (`self.PlayerControllers`) _asplayer_controller))

(event `self.ReceiveBeginPlay`
  (bind _returnvalue (`|CreateWidget` "/Game/Multiplayer/ProtoLobby/WG_Lobby.WG_Lobby_C"))
  (`UserWidget.AddToViewport` _returnvalue 0))

(event `self.HandleStartingNewPlayer`
  (params (NewPlayer :type "PlayerController Object Reference"))
  (`KismetSystemLibrary.PrintString` "Player Incomming" true true (struct :`G` 0.66 :`B` 1.0 :`A` 1.0) 5.0 "bite")
  (`KismetArrayLibrary.Array_AddUnique` (`self.PlayerControllers`) NewPlayer)
  (`KismetSystemLibrary.RetriggerableDelay` 0.2)
  (bind (_numconnections _numprivateconnections _bislan _bisdedicated _ballowinvites _ballowjoininprogress _bisanticheatenabled _builduniqueid _extrasettings) (`AdvancedSessionsLibrary.GetSessionSettings`)
    (:`OnSuccess`
      (`KismetSystemLibrary.PrintString` (`KismetStringLibrary.Concat_StrStr` "NB Player Controller : " (`KismetStringLibrary.Conv_IntToString` (`KismetArrayLibrary.Array_Length` (`self.PlayerControllers`)))) true true (struct :`R` 0.144346 :`G` 0.4375 :`A` 1.0) 2.0 "NBP")
      (`KismetSystemLibrary.PrintString` (`KismetStringLibrary.Concat_StrStr` "NB Connexion :" (`KismetStringLibrary.Conv_IntToString` _numconnections)) true true (struct :`R` 0.3125 :`G` 0.050623 :`B` 0.20284 :`A` 1.0) 2.0 "ServLenght")
      (if (> (`KismetArrayLibrary.Array_Length` (`self.PlayerControllers`)) _numconnections)
        (bind (_arrayindex _arrayelement) (`/Engine/EditorBlueprintResources/StandardMacros.ReverseForEachLoop` (`self.PlayerControllers`))
          (:`LoopBody`
            (if (>= _arrayindex _numconnections)
              (`AdvancedSessionsLibrary.KickPlayer` _arrayelement "Serveur complet")))
          (:`Completed`
            (`UpdateSessionCallbackProxyAdvanced.UpdateSession` _extrasettings _numconnections :!label _label)))
        (elif (== (`KismetArrayLibrary.Array_Length` (`self.PlayerControllers`)) _numconnections)
          (`KismetSystemLibrary.PrintString` "Everyone is here" true true (struct :`R` 1.0 :`B` 0.034397 :`A` 1.0) 5.0 "okogkggodfgd")
          (goto _label))))))

(fn `UserConstructionScript`)