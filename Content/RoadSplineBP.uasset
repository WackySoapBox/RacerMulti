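; RoadSplineBP is a road spline Blueprint meant to lay spline mesh segments along its Spline component.
; Its loop adds a SplineMeshComponent per pair of neighboring points, attaches it to DefaultSceneRoot and shapes it from both points' local locations and tangents.
; That loop is disconnected from the empty Construction Script, so this graph currently generates no segments.
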(fn `UserConstructionScript`)