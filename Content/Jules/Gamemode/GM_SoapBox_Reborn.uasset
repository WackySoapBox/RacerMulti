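; Game mode for a soapbox vehicle race that runs the start countdown and hands control to the player.
; On BeginPlay it shows a countdown widget, timing the 3-2-1 and "Let's Go" elements through delays and opacity changes.
; At "Let's Go" it clears FreezeStart on the first player's PC_Vehicle pawn.
; A second later it removes all widgets and adds the placement widget.
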(event `self.ReceiveBeginPlay`
  (bind _returnvalue (`|CreateWidget` "/Game/Jules/UI/Widgets/WG_StartCountdown.WG_StartCountdown_C"))
  (`UserWidget.AddToViewport` _returnvalue 0)
  (`Image.SetOpacity` (`/Game/Jules/UI/Widgets/WG_StartCountdown.num3` _returnvalue) 0.0)
  (`Image.SetOpacity` (`/Game/Jules/UI/Widgets/WG_StartCountdown.num2` _returnvalue) 0.0)
  (`Image.SetOpacity` (`/Game/Jules/UI/Widgets/WG_StartCountdown.num1` _returnvalue) 0.0)
  (`Image.SetOpacity` (`/Game/Jules/UI/Widgets/WG_StartCountdown.LetsGo` _returnvalue) 0.0)
  (`KismetSystemLibrary.Delay` 0.2)
  (`Image.SetOpacity` (`/Game/Jules/UI/Widgets/WG_StartCountdown.num3` _returnvalue) 1.0)
  (`KismetSystemLibrary.Delay` 1.0)
  (`Image.SetOpacity` (`/Game/Jules/UI/Widgets/WG_StartCountdown.num2` _returnvalue) 1.0)
  (`KismetSystemLibrary.Delay` 1.0)
  (`Image.SetOpacity` (`/Game/Jules/UI/Widgets/WG_StartCountdown.num1` _returnvalue) 1.0)
  (`KismetSystemLibrary.Delay` 1.0)
  (`Image.SetOpacity` (`/Game/Jules/UI/Widgets/WG_StartCountdown.num3` _returnvalue) 0.0)
  (`Image.SetOpacity` (`/Game/Jules/UI/Widgets/WG_StartCountdown.num2` _returnvalue) 0.0)
  (`Image.SetOpacity` (`/Game/Jules/UI/Widgets/WG_StartCountdown.num1` _returnvalue) 0.0)
  (`Image.SetOpacity` (`/Game/Jules/UI/Widgets/WG_StartCountdown.LetsGo` _returnvalue) 1.0)
  (bind _aspc_vehicle (cast `/Game/Jules/Pawn/PC_Vehicle` (`GameplayStatics.GetPlayerPawn` 0)))
  (set `/Game/Jules/Pawn/PC_Vehicle.freezeStart` false _aspc_vehicle)
  (`KismetSystemLibrary.Delay` 1.0)
  (`Image.SetOpacity` (`/Game/Jules/UI/Widgets/WG_StartCountdown.LetsGo` _returnvalue) 0.0)
  (`WidgetLayoutLibrary.RemoveAllWidgets`)
  (bind _returnvalue_2 (`|CreateWidget` "/Game/Jules/UI/Widgets/WG_Placement.WG_Placement_C" (`GameplayStatics.GetPlayerController` 0)))
  (`UserWidget.AddToViewport` _returnvalue_2 0))

(fn `UserConstructionScript`)