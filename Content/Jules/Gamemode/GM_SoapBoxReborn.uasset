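; Game mode for the SoapBox racing game that runs the race start countdown and assigns spawn points.
; Shortly after BeginPlay, a delay-driven countdown widget shows 3-2-1 and "Let's Go", sets FreezeStart on player 0's PC_Vehicle pawn, then swaps to the placement widget.
; ChoosePlayerStart finds the player's index in GI_Racer's ArrayPC and returns the start named index plus one, printing debug strings.
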(event `Count Down On Server`
  (`self.Count Down On Client` :!label _label))

(event `Count Down On Client`
  (bind _returnvalue (`|CreateWidget` "/Game/Jules/UI/Widgets/WG_StartCountdown.WG_StartCountdown_C"))
  (`UserWidget.AddToViewport` _returnvalue 0)
  (`KismetSystemLibrary.Delay` 1.0)
  (`Image.SetOpacity` (`/Game/Jules/UI/Widgets/WG_StartCountdown.num3` _returnvalue) 0.0)
  (`Image.SetOpacity` (`/Game/Jules/UI/Widgets/WG_StartCountdown.num2` _returnvalue) 0.0)
  (`Image.SetOpacity` (`/Game/Jules/UI/Widgets/WG_StartCountdown.num1` _returnvalue) 0.0)
  (`Image.SetOpacity` (`/Game/Jules/UI/Widgets/WG_StartCountdown.LetsGo` _returnvalue) 0.0)
  (`KismetSystemLibrary.Delay` 0.2)
  (`Image.SetOpacity` (`/Game/Jules/UI/Widgets/WG_StartCountdown.num3` _returnvalue) 1.0)
  (`KismetSystemLibrary.Delay` 1.0)
  (`Image.SetOpacity` (`/Game/Jules/UI/Widgets/WG_StartCountdown.num2` _returnvalue) 1.0)
  (`KismetSystemLibrary.Delay` 1.0)
  (`Image.SetOpacity` (`/Game/Jules/UI/Widgets/WG_StartCountdown.num1` _returnvalue) 1.0)
  (`KismetSystemLibrary.Delay` 1.0)
  (`Image.SetOpacity` (`/Game/Jules/UI/Widgets/WG_StartCountdown.num3` _returnvalue) 0.0)
  (`Image.SetOpacity` (`/Game/Jules/UI/Widgets/WG_StartCountdown.num2` _returnvalue) 0.0)
  (`Image.SetOpacity` (`/Game/Jules/UI/Widgets/WG_StartCountdown.num1` _returnvalue) 0.0)
  (`Image.SetOpacity` (`/Game/Jules/UI/Widgets/WG_StartCountdown.LetsGo` _returnvalue) 1.0)
  (bind _aspc_vehicle (cast `/Game/Jules/Pawn/PC_Vehicle` (`GameplayStatics.GetPlayerPawn` 0)))
  (set `/Game/Jules/Pawn/PC_Vehicle.freezeStart` true _aspc_vehicle)
  (`KismetSystemLibrary.Delay` 1.0)
  (`Image.SetOpacity` (`/Game/Jules/UI/Widgets/WG_StartCountdown.LetsGo` _returnvalue) 0.0)
  (`WidgetLayoutLibrary.RemoveAllWidgets`)
  (bind _returnvalue_2 (`|CreateWidget` "/Game/Jules/UI/Widgets/WG_Placement.WG_Placement_C"))
  (`UserWidget.AddToViewport` _returnvalue_2 0))

(event `self.ReceiveBeginPlay`
  (`KismetSystemLibrary.Delay` 1.0)
  (goto _label))

(fn `ChoosePlayerStart`
  (params (Player :type "Controller Object Reference"))
  (returns (ReturnValue :type "Actor Object Reference"))
  (`KismetSystemLibrary.PrintString` (`KismetSystemLibrary.GetDisplayName` Player) true true (struct :`G` 0.004274 :`B` 1.0 :`A` 1.0) 25.0)
  (bind _asgi_racer (cast `/Game/Multiplayer/Menu/GI_Racer` (`GameplayStatics.GetGameInstance`)))
  (for (_array_element _array_index) (`/Game/Multiplayer/Menu/GI_Racer.Array_PC` _asgi_racer)
    (bind _returnvalue (+ _array_index 1))
    (`KismetSystemLibrary.PrintString` (`KismetStringLibrary.Concat_StrStr` "Player : " (`KismetSystemLibrary.GetDisplayName` _array_element) "| index spawn : " (`KismetStringLibrary.Conv_IntToString` _returnvalue) "| tab index :" (`KismetStringLibrary.Conv_IntToString` _array_index)) true true (struct :`G` 0.66 :`B` 1.0 :`A` 1.0) 15.0 (`KismetStringLibrary.Conv_StringToName` (`KismetStringLibrary.Conv_IntToString` _array_index)))
    (if (== _array_element Player)
      (bind _returnvalue_2 (`self.K2_FindPlayerStart` Player (`KismetStringLibrary.Conv_IntToString` _returnvalue)))
      (`KismetSystemLibrary.PrintString` (`KismetSystemLibrary.GetDisplayName` _returnvalue_2) true true (struct :`R` 0.921582 :`G` 0.000304 :`B` 0.610496 :`A` 1.0) 20.0 "playerstart")
      (return _returnvalue_2)))
  (`KismetSystemLibrary.PrintString` (`KismetStringLibrary.Conv_IntToString` _array_index) true true (struct :`G` 0.66 :`B` 1.0 :`A` 1.0) 22.0))

(fn `CountDown on Server`)

(fn `UserConstructionScript`)