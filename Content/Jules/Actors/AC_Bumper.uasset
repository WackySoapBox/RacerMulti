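; AC_Bumper is a bumper actor that reacts to overlaps with actors tagged Player by attempting to push them.
; On overlap it prints the actor's name and adds a force to that actor's primitive components.
; The force is the scaled offset from player pawn 0 to the overlapping actor, not from the bumper, so it is zero when that pawn itself overlaps.
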(event `self.ReceiveActorBeginOverlap`
  (params (OtherActor :type "Actor Object Reference"))
  (if (`self.ActorHasTag` OtherActor "Player")
    (`KismetSystemLibrary.PrintString` (`KismetSystemLibrary.GetDisplayName` OtherActor))
    (`PrimitiveComponent.AddForce` (`self.K2_GetComponentsByClass` OtherActor "/Script/Engine.PrimitiveComponent") (* (- (`self.K2_GetActorLocation` OtherActor) (`self.K2_GetActorLocation` (`GameplayStatics.GetPlayerPawn` 0))) (20.0 20.0 20.0)) "None" false)))

(fn `UserConstructionScript`)