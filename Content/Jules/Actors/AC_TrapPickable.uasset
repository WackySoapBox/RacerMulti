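; Throwable trap pickup actor that can hit player vehicles.
; Thrown stores a direction, and Tick then makes a swept move each frame to 200 units along it from the Sphere's current location.
; Sphere1 overlap with a Player-tagged PC_Vehicle calls Touched and destroys the trap, but only if IsActivated, which is set only in disconnected debug logic.
; Hit, PickedUp and component-hit handlers are empty.
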(event `self.ReceiveHit`
  (params (MyComp :type "PrimitiveComponent Object Reference") (Other :type "Actor Object Reference") (OtherComp :type "PrimitiveComponent Object Reference") (bSelfMoved :type Boolean) (HitLocation :type "Vector Structure") (HitNormal :type "Vector Structure") (NormalImpulse :type "Vector Structure") (Hit :type "HitResult Structure (by ref)")))

(event `PickedUp`
  (params (Player :type "/Game/Jules/Pawn/PC_Vehicle Object Reference")))

(event `Thrown`
  (params (VectorForward :type "Vector Structure"))
  (set `self.isThrown` true)
  (set `self.vectorToFollow` VectorForward))

(event `self.ReceiveTick`
  (params (DeltaSeconds :type "Float (single-precision)"))
  (if (`self.isThrown`)
    (`self.K2_SetActorLocation` (+ (`SceneComponent.K2_GetComponentLocation` (`self.Sphere`)) (* (`self.vectorToFollow`) (200.0 200.0 200.0))) true)))

(event `self.Sphere1.OnComponentHit`
  (params (HitComponent :type "PrimitiveComponent Object Reference") (OtherActor :type "Actor Object Reference") (OtherComp :type "PrimitiveComponent Object Reference") (NormalImpulse :type "Vector Structure") (Hit :type "HitResult Structure (by ref)")))

(event `self.Sphere1.OnComponentBeginOverlap`
  (params (OverlappedComponent :type "PrimitiveComponent Object Reference") (OtherActor :type "Actor Object Reference") (OtherComp :type "PrimitiveComponent Object Reference") (OtherBodyIndex :type Integer) (bFromSweep :type Boolean) (SweepResult :type "HitResult Structure (by ref)"))
  (if (`self.ActorHasTag` OtherActor "Player")
    (if (`self.isActivated`)
      (bind _aspc_vehicle (cast `/Game/Jules/Pawn/PC_Vehicle` OtherActor))
      (`/Game/Jules/Pawn/PC_Vehicle.Touched` _aspc_vehicle)
      (`self.K2_DestroyActor`))))

(fn `UserConstructionScript`)