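; AC_Player_Test is a test actor that experiments with physics impulses on its Cube component.
; Overlapping an actor tagged "Pickable" launches the Cube upward, while BumpYourself shoves it along negative Y, both as velocity changes.
; Box overlaps only print the other actor's name, and TakeMyForce stores a ProjectionForce that nothing here reads.
; A disconnected force and impulse test chain never runs.
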(event `self.Box.OnComponentBeginOverlap`
  (params (OverlappedComponent :type "PrimitiveComponent Object Reference") (OtherActor :type "Actor Object Reference") (OtherComp :type "PrimitiveComponent Object Reference") (OtherBodyIndex :type Integer) (bFromSweep :type Boolean) (SweepResult :type "HitResult Structure (by ref)"))
  (`KismetSystemLibrary.PrintString` (`KismetSystemLibrary.GetDisplayName` OtherActor)))

(event `BumpYourself`
  (`PrimitiveComponent.AddImpulse` (`self.Cube`) (0.0 -1000.0 0.0) "None" true))

(event `self.ReceiveActorBeginOverlap`
  (params (OtherActor :type "Actor Object Reference"))
  (if (`self.ActorHasTag` OtherActor "Pickable")
    (`PrimitiveComponent.AddImpulse` (`self.Cube`) (0.0 0.0 2000.0) "None" true)))

(event `TakeMyForce`
  (params (Force :type "Vector Structure"))
  (set `self.projectionForce` Force))

(fn `UserConstructionScript`)