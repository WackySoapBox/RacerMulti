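; AC_Cart is a cart pickup actor that gives the player's suspension test pawn another cart when touched.
; On overlap with a "Player"-tagged actor, it casts to PC_Test_suspension and calls AddCart.
; It then hides its ground and four walls and disables their collision, restoring visibility and query-only collision after a half-second delay, so it acts as a quickly respawning pickup.
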(event `self.ReceiveActorBeginOverlap`
  (params (OtherActor :type "Actor Object Reference"))
  (if (`self.ActorHasTag` OtherActor "Player")
    (bind _aspc_test_suspension (cast `/Game/Jules/Pawn/PC_Test_suspension` OtherActor))
    (`/Game/Jules/Pawn/PC_Test_suspension.AddCart` _aspc_test_suspension)
    (`SceneComponent.SetVisibility` (`self.Ground`) false false)
    (`SceneComponent.SetVisibility` (`self.Wall1`) false false)
    (`SceneComponent.SetVisibility` (`self.Wall2`) false false)
    (`SceneComponent.SetVisibility` (`self.Wall3`) false false)
    (`SceneComponent.SetVisibility` (`self.Wall4`) false false)
    (`PrimitiveComponent.SetCollisionEnabled` (`self.Ground`) "NoCollision")
    (`PrimitiveComponent.SetCollisionEnabled` (`self.Wall1`) "NoCollision")
    (`PrimitiveComponent.SetCollisionEnabled` (`self.Wall2`) "NoCollision")
    (`PrimitiveComponent.SetCollisionEnabled` (`self.Wall3`) "NoCollision")
    (`PrimitiveComponent.SetCollisionEnabled` (`self.Wall4`) "NoCollision")
    (`KismetSystemLibrary.Delay` 0.5)
    (`SceneComponent.SetVisibility` (`self.Ground`) true false)
    (`SceneComponent.SetVisibility` (`self.Wall1`) true false)
    (`SceneComponent.SetVisibility` (`self.Wall2`) true false)
    (`SceneComponent.SetVisibility` (`self.Wall3`) true false)
    (`SceneComponent.SetVisibility` (`self.Wall4`) true false)
    (`PrimitiveComponent.SetCollisionEnabled` (`self.Ground`) "QueryOnly")
    (`PrimitiveComponent.SetCollisionEnabled` (`self.Wall1`) "QueryOnly")
    (`PrimitiveComponent.SetCollisionEnabled` (`self.Wall2`) "QueryOnly")
    (`PrimitiveComponent.SetCollisionEnabled` (`self.Wall3`) "QueryOnly")
    (`PrimitiveComponent.SetCollisionEnabled` (`self.Wall4`) "QueryOnly")))

(fn `UserConstructionScript`)