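; AC_MysteryBoxPickable is a mystery box pickup for vehicles that spins continuously on Tick.
; When an actor tagged Player overlaps it, it casts that actor to PC_Vehicle and calls GotMysteryBox.
; It then hides and disables collision on the MysteryBox component, and restores both after a short Delay so the pickup can be collected again.
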(event `self.ReceiveTick`
  (params (DeltaSeconds :type "Float (single-precision)"))
  ;[1 1 1] Rotation
  (`SceneComponent.K2_AddLocalRotation` (`self.Cube`) (struct :`Pitch` 1.0 :`Yaw` 1.0 :`Roll` 1.0) false false))

(event `self.ReceiveActorBeginOverlap`
  (params (OtherActor :type "Actor Object Reference"))
  ;[1 1 1] On contact w/Player
  (if (`self.ActorHasTag` OtherActor "Player")
    (bind _aspc_vehicle (cast `/Game/Jules/Pawn/PC_Vehicle` OtherActor))
    (`/Game/Jules/Pawn/PC_Vehicle.GotMysteryBox` _aspc_vehicle)
    (`PrimitiveComponent.SetCollisionEnabled` (`self.MysteryBox`) "NoCollision")
    (`SceneComponent.SetVisibility` (`self.MysteryBox`) false false)
    (`KismetSystemLibrary.Delay` 1.0)
    (`SceneComponent.SetVisibility` (`self.MysteryBox`) true false)
    (`PrimitiveComponent.SetCollisionEnabled` (`self.MysteryBox`) "QueryOnly")))

(fn `UserConstructionScript`)