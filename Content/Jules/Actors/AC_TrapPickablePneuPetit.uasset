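; Small tire ("pneu petit") trap pickup that can be thrown to push players.
; Thrown arms it and stores direction and rotation; overlapping a player while armed passes VectorForce to TakeMyForce, then destroys it shortly after.
; Pickup destroys the actor, and left/right bump events both apply the given impulse to the Dur component.
; Player hits play a 2D sound, gated by a DoOnce until it ends.
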(event `self.ReceiveActorBeginOverlap`
  (params (OtherActor :type "Actor Object Reference"))
  (if (and (`self.ActorHasTag` OtherActor "Player") (`self.isThrown`))
    (bind _asac_player_test (cast `/Game/Jules/Actors/AC_Player_Test` OtherActor))
    (`/Game/Jules/Actors/AC_Player_Test.TakeMyForce` _asac_player_test (`self.vectorForce`))
    (`KismetSystemLibrary.Delay` 0.2)
    (`self.K2_DestroyActor`)))

(event `Thrown`
  (params (VectorForward :type "Vector Structure") (Rot :type "Rotator Structure"))
  (set `self.isThrown` true)
  (set `self.vectorToFollow` VectorForward)
  (set `self.RotToHave` Rot))

(event `PickedUp`
  (params (Player :type "/Game/Jules/Pawn/PC_Vehicle Object Reference"))
  (`self.K2_DestroyActor`))

(event `BumpYourselfRight`
  (params (Force :type "Vector Structure"))
  (`PrimitiveComponent.AddImpulse` (`self.Dur`) Force "None" false))

(event `BumpYourselfLeft`
  (params (Force :type "Vector Structure"))
  (`PrimitiveComponent.AddImpulse` (`self.Dur`) Force "None" false))

(event `self.ReceiveHit`
  (params (MyComp :type "PrimitiveComponent Object Reference") (Other :type "Actor Object Reference") (OtherComp :type "PrimitiveComponent Object Reference") (bSelfMoved :type Boolean) (HitLocation :type "Vector Structure") (HitNormal :type "Vector Structure") (NormalImpulse :type "Vector Structure") (Hit :type "HitResult Structure (by ref)"))
  (bind _sound (`self.Sound`))
  (`/Engine/EditorBlueprintResources/StandardMacros.DoOnce` false :!label _label
    (:`Completed`
      (if (`self.ActorHasTag` Hit_HitActor "Player")
        (`GameplayStatics.SpawnSound2D` _sound 1.0 1.0 0.0 null)
        (`KismetSystemLibrary.Delay` (`SoundBase.Duration` _sound))
        (goto _label :!via `Reset`)
        (else
          (goto _label :!via `Reset`))))))

(fn `UserConstructionScript`)