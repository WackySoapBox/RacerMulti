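; AC_LostPart is a pickup for a lost part that a player's PC_Vehicle collects by driving into it.
; ChangeStaticMesh stores and shows the given mesh, then enables pickup after a short delay.
; On overlap with a Player-tagged actor once that cooldown is done, it passes the mesh to the vehicle's IntegratePickedUpLostPart and destroys itself.
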(event `ChangeStaticMesh`
  (params (StaticMesh :type "StaticMesh Object Reference"))
  (bind _sm_lostpart (`self.SM_LostPart`))
  (set `self.CurrentMeshHolding` StaticMesh)
  (`StaticMeshComponent.SetStaticMesh` _sm_lostpart StaticMesh)
  (`SceneComponent.SetVisibility` _sm_lostpart true false)
  (`KismetSystemLibrary.Delay` 0.2)
  (set `self.CooldownDone` true))

(event `self.ReceiveActorBeginOverlap`
  (params (OtherActor :type "Actor Object Reference"))
  (if (`self.ActorHasTag` OtherActor "Player")
    (if (`self.CooldownDone`)
      (bind _aspc_vehicle (cast `/Game/Jules/Pawn/PC_Vehicle` OtherActor))
      (`/Game/Jules/Pawn/PC_Vehicle.IntegratePickedUpLostPart` _aspc_vehicle (`self.CurrentMeshHolding`))
      (`self.K2_DestroyActor`))))

(fn `UserConstructionScript`)