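; Panel actor for an in-world 3D menu that pairs a host/join (Héberger/Rejoindre) switch widget with separate hosting and joining widget components.
; On BeginPlay it passes both components to the WG_3D_SwitchHébergerRejoindre widget, then hides their user widgets.
; The Blueprint holds no switching logic itself, and a click on the hosting component only prints a debug string.
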(event `self.ReceiveBeginPlay`
  (bind _widgethebergement (`self.WidgetHebergement`))
  (bind _widgetrejoindre (`self.WidgetRejoindre`))
  (bind `_aswg_3d_switch_héberger_rejoindre` (cast `/Game/UI/Widgets/WG_3D_SwitchHébergerRejoindre` (`WidgetComponent.GetUserWidgetObject` (`self.WidgetSwitch`))))
  (set `/Game/UI/Widgets/WG_3D_SwitchHébergerRejoindre.WidgetHebergement` _widgethebergement `_aswg_3d_switch_héberger_rejoindre`)
  (set `/Game/UI/Widgets/WG_3D_SwitchHébergerRejoindre.WidgetRejoindre` _widgetrejoindre `_aswg_3d_switch_héberger_rejoindre`)
  (`Widget.SetVisibility` (`WidgetComponent.GetUserWidgetObject` _widgetrejoindre) "Hidden")
  (`Widget.SetVisibility` (`WidgetComponent.GetUserWidgetObject` _widgethebergement) "Hidden"))

(event `self.WidgetHebergement.OnClicked`
  (params (TouchedComponent :type "PrimitiveComponent Object Reference") (ButtonPressed :type "Key Structure"))
  (`KismetSystemLibrary.PrintString` "bonsoiro" true true (struct :`G` 0.66 :`B` 1.0 :`A` 1.0) 2.0 "Nfdghgjhone"))

(fn `UserConstructionScript`)