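; BP_Panneau1 is a 3D menu sign prop with three text widget components: Jouer, Entrainement and Crédits.
; BeginPlay labels and colors each WG_3D_MenuText through SetupWidget, collects them in ListWidget and shows the mouse cursor.
; Selected and NotSelected events recolor a passed widget component to show highlight state.
; Tick prints the Jouer widget's text and world location as debug output.
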(event `Selected`
  (params (NewParam :type "WidgetComponent Object Reference"))
  (bind _aswg_3d_menu_text (cast `/Game/UI/Widgets/WG_3D_MenuText` (`WidgetComponent.GetUserWidgetObject` NewParam)))
  (set `/Game/UI/Widgets/WG_3D_MenuText.color` (`self.ColorSelected`) _aswg_3d_menu_text))

(event `NotSelected`
  (params (NewParam :type "WidgetComponent Object Reference"))
  (bind _aswg_3d_menu_text (cast `/Game/UI/Widgets/WG_3D_MenuText` (`WidgetComponent.GetUserWidgetObject` NewParam)))
  (set `/Game/UI/Widgets/WG_3D_MenuText.color` (`self.ColorUnselected`) _aswg_3d_menu_text))

(event `self.ReceiveBeginPlay`
  (bind _listwidget (`self.ListWidget`))
  (`KismetArrayLibrary.Array_Clear` _listwidget)
  (`self.SetupWidget` (`WidgetComponent.GetUserWidgetObject` (`self.WidgetJouer`)) (`self.ColorUnselected`) (`|FormatText` "Jouer") _listwidget)
  (`self.SetupWidget` (`WidgetComponent.GetUserWidgetObject` (`self.WidgetEntrainement`)) (`self.ColorUnselected`) (`|FormatText` "Entrainement") _listwidget)
  (`self.SetupWidget` (`WidgetComponent.GetUserWidgetObject` (`self.WidgetCrédits`)) (`self.ColorUnselected`) (`|FormatText` "Crédits") _listwidget)
  (set `PlayerController.bShowMouseCursor` true (`GameplayStatics.GetPlayerController` 0)))

(event `self.ReceiveTick`
  (params (DeltaSeconds :type "Float (single-precision)"))
  (bind _widgetjouer (`self.WidgetJouer`))
  (bind _aswg_3d_menu_text (cast `/Game/UI/Widgets/WG_3D_MenuText` (`WidgetComponent.GetUserWidgetObject` _widgetjouer)))
  (`KismetSystemLibrary.PrintString` (`KismetStringLibrary.Concat_StrStr` (`KismetTextLibrary.Conv_TextToString` (`/Game/UI/Widgets/WG_3D_MenuText.Text` _aswg_3d_menu_text)) " |" (`KismetStringLibrary.Conv_VectorToString` (`SceneComponent.K2_GetComponentLocation` _widgetjouer))) true true (struct :`G` 0.66 :`B` 1.0 :`A` 1.0) 2.0 "dzaaddzazdazdazd"))

(fn `SetupWidget`
  (params (Widget :type "UserWidget Object Reference") (Color :type "LinearColor Structure") (Text :type Text) (ListWidget :type "Array of /Game/UI/Widgets/WG_3D_MenuText Object Reference"))
  (bind _aswg_3d_menu_text (cast `/Game/UI/Widgets/WG_3D_MenuText` Widget))
  (`KismetArrayLibrary.Array_AddUnique` ListWidget _aswg_3d_menu_text)
  (set `/Game/UI/Widgets/WG_3D_MenuText.text` Text _aswg_3d_menu_text)
  (set `/Game/UI/Widgets/WG_3D_MenuText.color` Color _aswg_3d_menu_text))

(fn `UserConstructionScript`)