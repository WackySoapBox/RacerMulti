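; BP_bottedepaille2 is a hay bale that reacts when an actor tagged Player touches it.
; Overlapping the main collider plays a timeline from the start, driving a morph target on the skeletal mesh to deform the bale.
; Overlapping the separate BP_jump volume enables physics on the mesh and launches it forward along X and upward, with random sideways velocity.
; The collider's end-overlap only checks the tag and has no effect.
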(event `self.Botte_paille_collider.OnComponentBeginOverlap`
  (params (OverlappedComponent :type "PrimitiveComponent Object Reference") (OtherActor :type "Actor Object Reference") (OtherComp :type "PrimitiveComponent Object Reference") (OtherBodyIndex :type Integer) (bFromSweep :type Boolean) (SweepResult :type "HitResult Structure (by ref)"))
  (if (`self.ActorHasTag` OtherActor "Player")
    (bind (_direction _newtrack_0) (`Timeline|Timeline_BP` :!via `PlayFromStart`)
      (:`Update`
        (`SkeletalMeshComponent.SetMorphTarget` (`self.BP_skeletal`) "Botte_de_paille_03" _newtrack_0 true)
        (`/Engine/EditorBlueprintResources/StandardMacros.DoOnce` false)))))

(event `self.Botte_paille_collider.OnComponentEndOverlap`
  (params (OverlappedComponent :type "PrimitiveComponent Object Reference") (OtherActor :type "Actor Object Reference") (OtherComp :type "PrimitiveComponent Object Reference") (OtherBodyIndex :type Integer))
  (if (`self.ActorHasTag` OtherActor "Player")
    _))

(event `self.BP_jump.OnComponentBeginOverlap`
  (params (OverlappedComponent :type "PrimitiveComponent Object Reference") (OtherActor :type "Actor Object Reference") (OtherComp :type "PrimitiveComponent Object Reference") (OtherBodyIndex :type Integer) (bFromSweep :type Boolean) (SweepResult :type "HitResult Structure (by ref)"))
  (if (`self.ActorHasTag` OtherActor "Player")
    (`PrimitiveComponent.SetSimulatePhysics` (`self.BP_skeletal`) true)
    (`PrimitiveComponent.SetPhysicsLinearVelocity` (`self.BP_skeletal`) (`KismetMathLibrary.MakeVector` 400.0 (`KismetMathLibrary.RandomFloatInRange` -400.0 400.0) 400.0) true "None")))

(fn `UserConstructionScript`)