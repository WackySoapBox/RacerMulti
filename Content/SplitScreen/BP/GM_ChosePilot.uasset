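; Game mode for split-screen pilot selection, spawning one local player per player count stored in the GI_Racer game instance.
; On BeginPlay it creates players until the NbJoueur counter reaches that count, naming each "P" plus the counter.
; The counter advances inside the ChoosePlayerStart override, which sends each player to the PlayerStart whose tag matches the new number.
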(event `self.ReceiveBeginPlay`
  (bind _asgi_racer (cast `/Game/Multiplayer/Menu/GI_Racer` (`GameplayStatics.GetGameInstance`)))
  (bind _ss_numplayer (`/Game/Multiplayer/Menu/GI_Racer.SS_NumPlayer` _asgi_racer))
  (for _ (range (+ _ss_numplayer 1)) :!label _label
    (if (< (`self.NbJoueur`) _ss_numplayer)
      (bind _returnvalue (`GameplayStatics.CreatePlayer` -1))
      (`AdvancedSessionsLibrary.SetPlayerName` _returnvalue (`KismetStringLibrary.Concat_StrStr` "P" (`KismetStringLibrary.Conv_IntToString` (`self.NbJoueur`))))
      (else
        (`self.StopFor`)))))

(event `Stop For`
  (goto _label :!via `Break`))

(fn `ChoosePlayerStart`
  (params (Player :type "Controller Object Reference"))
  (returns (ReturnValue :type "Actor Object Reference"))
  (bind _output_get (set `self.NbJoueur` (+ (`self.NbJoueur`) 1)))
  (return (`self.K2_FindPlayerStart` null (`KismetStringLibrary.Conv_IntToString` _output_get))))

(fn `StopFor`)

(fn `UserConstructionScript`)