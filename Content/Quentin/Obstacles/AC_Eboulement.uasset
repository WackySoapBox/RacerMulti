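; AC_Eboulement is a rockslide obstacle that continuously spews rock actors from its Sphere component.
; Tick accumulates time and, each DelaySpawn interval, spawns an AC_Caillou at the Sphere with random non-uniform scale based on OffsetScale.
; Each rock's MSRocher mesh then gets a random physics velocity against the Sphere's forward vector, multiplied by Force.
; A player-triggered burst of overhead rocks remains in the graph but is disconnected.
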(event `self.ReceiveActorBeginOverlap`
  (params (OtherActor :type "Actor Object Reference")))

(event `self.ReceiveTick`
  (params (DeltaSeconds :type "Float (single-precision)"))
  (bind _returnvalue (* (`KismetMathLibrary.FMax` (`KismetMathLibrary.RandomFloat`) 0.5) (`self.OffsetScale`)))
  (bind _output_get (set `self.DelayPassed` (+ DeltaSeconds (`self.DelayPassed`))))
  (if (>= _output_get (`self.DelaySpawn`))
    (set `self.DelayPassed` 0.0)
    (bind _returnvalue_2 (`|SpawnActorFromClass` "/Game/Quentin/Obstacles/AC_Caillou.AC_Caillou_C" (`KismetMathLibrary.MakeTransform` (`SceneComponent.K2_GetComponentLocation` (`self.Sphere`)) (struct) (`KismetMathLibrary.MakeVector` _returnvalue _returnvalue _returnvalue)) "Undefined" "OverrideRootScale" null null))
    (`PrimitiveComponent.SetPhysicsLinearVelocity` (`/Game/Quentin/Obstacles/AC_Caillou.MS_Rocher` _returnvalue_2) (* (* (`SceneComponent.GetForwardVector` (`self.Sphere`)) (`KismetMathLibrary.RandomFloatInRange` -1750.0 -2250.0)) (`self.Force`)) true "None")))

(fn `UserConstructionScript`)