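; AC_Caillou is a short-lived rock obstacle actor that destroys itself five seconds after it begins play.
; Each overlap on the rock mesh spawns a rockslide sound (SC_Eboulement) attached to it.
; An unconnected branch would give the mesh a one-time downward velocity boost once it stops rising, but it never runs, and Tick is empty.
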(event `self.ReceiveTick`
  (params (DeltaSeconds :type "Float (single-precision)")))

(event `self.MS_Rocher.OnComponentBeginOverlap`
  (params (OverlappedComponent :type "PrimitiveComponent Object Reference") (OtherActor :type "Actor Object Reference") (OtherComp :type "PrimitiveComponent Object Reference") (OtherBodyIndex :type Integer) (bFromSweep :type Boolean) (SweepResult :type "HitResult Structure (by ref)"))
  (if true
    (`GameplayStatics.SpawnSoundAttached` "/Game/Jules/SoundDesign/SoundCues/SC_Eboulement.SC_Eboulement" (`self.MS_Rocher`) "None" (0.0 0.0 0.0) (struct) "KeepRelativeOffset" false 1.0 1.0 0.0 null null)))

(event `self.ReceiveBeginPlay`
  (`KismetSystemLibrary.Delay` 5.0)
  (`self.K2_DestroyActor`))

(fn `UserConstructionScript`)