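; BP_Controle is an actor that carries a WG_Controle widget and slides away when that widget's return button is pressed.
; On BeginPlay it gets the widget from its widget component and binds BTNRetour's press to RetourPress.
; RetourPress plays a timeline whose Temps track lerps from the current location toward a fixed offset, with sweep.
; Each update re-reads the location, so movement accumulates rather than ending at that offset.
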(event `self.ReceiveTick`
  (params (DeltaSeconds :type "Float (single-precision)")))

(event `self.ReceiveBeginPlay`
  (bind _aswg_controle (cast `/Game/UI/Widgets/WG_Controle` (`WidgetComponent.GetUserWidgetObject` (`self.WidgetControle`))))
  (add `Button.OnPressed` (`/Game/UI/Widgets/WG_Controle.BTN_Retour` _aswg_controle) (delegate `RetourPress`)))

(event `RetourPress`
  (bind _returnvalue (`self.K2_GetActorLocation`))
  (bind (_direction _temps) (`Timeline|Timeline` :!via `PlayFromStart`)
    (:`Update`
      (`self.K2_SetActorLocation` (`KismetMathLibrary.VLerp` _returnvalue (+ _returnvalue (-9.0 -7.0 0.0)) _temps) true))))

(fn `UserConstructionScript`)